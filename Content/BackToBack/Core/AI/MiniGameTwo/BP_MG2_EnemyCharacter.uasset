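; Enemy character for MiniGame Two that shows a floating health bar facing the top-down camera.
; BeginPlay finds and stores the BP_MG2_TopDownCamera actor in the level.
; Every Tick sets the HP bar widget's percent from CalculateHealthPercentage and rotates the widget component toward that camera, billboard-style.
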(event EventBeginPlay
  (bind _returnvalue (Actor|GetActorOfClass "/Game/BackToBack/Core/Camera/BP_MG2_TopDownCamera.BP_MG2_TopDownCamera_C"))
  (Variables|Default|SetMG2_TopDownCamera _returnvalue))

(event Collision|EventActorBeginOverlap
  (params (OtherActor :type Actor%20Object%20Reference)))

(event EventTick
  (params (DeltaSeconds :type Float%20%28single-precision%29))
  (bind _healthwidgetcomp (Variables|Default|GetHealthWidgetComp))
  ;[0 0 0] Updating Enemy Health Bar UI
  (bind _aswdp_mg2_enemy_hpbar_hud (Utilities|Casting|CastToWDP_MG2_EnemyHPBarHUD (UserInterface|GetWidget (Variables|Default|GetHealthWidgetComp))))
  (Progress|SetPercent (Variables|/Script/BackToBack.BTBEnemyHealthBarHUD|GetHPBar _aswdp_mg2_enemy_hpbar_hud) (Class|BTBEnemyCharacter|CalculateHealthPercentage))
  ;[0 0 0] Adjust Roation
  (Transformation|SetWorldRotation _healthwidgetcomp (Math|Rotator|FindLookatRotation (Transformation|GetWorldLocation _healthwidgetcomp) (Transformation|GetWorldLocation (Variables|/Script/BackToBack.BTBCamera|GetCamera (Variables|Default|GetMG2_TopDownCamera)))) false false))

(fn ConstructionScript)